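; MovingDoor is a door actor that the player can open only after collecting six orbs.
; Its box collision checks the overlapping MyCharacter's orb count, sets an on-screen prompt and enables input on the door when the count is met, then clears both on exit.
; The open-door input fires once, caching the starting rotation and playing a timeline that swings the whole actor in yaw.
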(event `self.ReceiveBeginPlay`)

(event `EnhancedInput|/Game/MyContent/Inputs/IA_OpenDoor`
  (params (ActionValue :type "Vector2D Structure") (ElapsedSeconds :type "Float (double-precision)") (TriggeredSeconds :type "Float (double-precision)") (InputAction :type "InputAction Object Reference" :default "/Game/MyContent/Inputs/IA_OpenDoor.IA_OpenDoor"))
  (:`Triggered`
    ; Door Rotation
    (`/Engine/EditorBlueprintResources/StandardMacros.DoOnce` false
      (:`Completed`
        (bind _output_get (set `self.InitialDoorRotation` (`self.K2_GetActorRotation`)))
        (bind (_direction _opendoormovement) (`Timeline|OpenDoorTimeline`)
          (:`Update`
            (`self.K2_SetActorRotation` (`KismetMathLibrary.MakeRotator` (.roll _output_get) (.pitch _output_get) (- (.yaw _output_get) _opendoormovement)))))))))

(event `self.BoxCollision.OnComponentBeginOverlap`
  (params (OverlappedComponent :type "PrimitiveComponent Object Reference") (OtherActor :type "Actor Object Reference") (OtherComp :type "PrimitiveComponent Object Reference") (OtherBodyIndex :type Integer) (bFromSweep :type Boolean) (SweepResult :type "HitResult Structure (by ref)"))
  ; Enable/ Disable input on door
  (bind _asmy_character (cast `/Game/MyContent/Blueprints/MyCharacter` OtherActor))
  (if (== (`/Game/MyContent/Blueprints/MyCharacter.OrbsCollected` _asmy_character) 6)
    (set `/Game/MyContent/Blueprints/MyCharacter.ScreenMessage` "Press F to Open the door" _asmy_character)
    (`self.EnableInput` (`GameplayStatics.GetPlayerController` 0))
    (else
      (set `/Game/MyContent/Blueprints/MyCharacter.ScreenMessage` "You must collect all the orbs to open this door" _asmy_character))))

(event `self.BoxCollision.OnComponentEndOverlap`
  (params (OverlappedComponent :type "PrimitiveComponent Object Reference") (OtherActor :type "Actor Object Reference") (OtherComp :type "PrimitiveComponent Object Reference") (OtherBodyIndex :type Integer))
  ; Enable/ Disable input on door
  (bind _asmy_character (cast `/Game/MyContent/Blueprints/MyCharacter` OtherActor))
  (set `/Game/MyContent/Blueprints/MyCharacter.ScreenMessage` "" _asmy_character)
  (`self.DisableInput` (`GameplayStatics.GetPlayerController` 0)))

(fn `UserConstructionScript`)