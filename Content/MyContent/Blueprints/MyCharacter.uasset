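; Player character Blueprint that manages health, the HUD and the win and game-over screens.
; BeginPlay adds the default Enhanced Input context, shows the HUD and pre-creates pause, game-over and win widgets.
; AnyDamage passes through a DoOnce reset after delays, giving brief invulnerability and a damage tint flag, and triggers game over at zero health.
; Both end events swap in their menu, switch to UI-only input with cursor, and pause.
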(event `self.ReceiveAnyDamage`
  (params (Damage :type "Float (single-precision)") (DamageType :type "DamageType Object Reference") (InstigatedBy :type "Controller Object Reference") (DamageCauser :type "Actor Object Reference"))
  ; Health y deducir vida
  (`/Engine/EditorBlueprintResources/StandardMacros.DoOnce` false :!label _label
    (:`Completed`
      (bind _output_get (set `self.Health` (- (`self.Health`) Damage)))
      (if (<= _output_get 0.001)
        (`self.Event GameOver`)
        (else
          (set `self.ShowDamageTint` true)
          (`KismetSystemLibrary.Delay` 0.2)
          (set `self.ShowDamageTint` false)
          (`KismetSystemLibrary.Delay` 0.3)
          (goto _label :!via `Reset`))))))

(event `EventWinGame`
  (bind _returnvalue (`GameplayStatics.GetPlayerController` 0))
  (bind _winscreenmenu (`self.WinScreenMenu`))
  ; WinGame
  (`WidgetLayoutLibrary.RemoveAllWidgets`)
  (`UserWidget.AddToViewport` _winscreenmenu 0)
  (`WidgetBlueprintLibrary.SetInputMode_UIOnlyEx` _returnvalue _winscreenmenu)
  (set `PlayerController.bShowMouseCursor` true _returnvalue)
  (`GameplayStatics.SetGamePaused` true))

(event `Event GameOver`
  (bind _returnvalue (`GameplayStatics.GetPlayerController` 0))
  (bind _gameovermenu (`self.GameOverMenu`))
  ; GameOver
  (`WidgetLayoutLibrary.RemoveAllWidgets`)
  (`UserWidget.AddToViewport` _gameovermenu 0)
  (`WidgetBlueprintLibrary.SetInputMode_UIOnlyEx` _returnvalue _gameovermenu)
  (set `PlayerController.bShowMouseCursor` true _returnvalue)
  (`GameplayStatics.SetGamePaused` true))

(event `self.ReceiveBeginPlay`
  ; Inputs y HUD
  (`EnhancedInputSubsystemInterface.AddMappingContext` (pcsubsystem `EnhancedInputLocalPlayerSubsystem` (`GameplayStatics.GetPlayerController` 0)) "/Game/MyContent/Inputs/IMC_Default.IMC_Default" 0 (struct))
  (bind _returnvalue (`|CreateWidget` "/Game/MyContent/HUD/MyHUD.MyHUD_C"))
  (bind _output_get (set `self.MyHUD` _returnvalue))
  (`UserWidget.AddToViewport` _output_get 0)
  (bind _returnvalue_2 (`|CreateWidget` "/Game/MyContent/HUD/PauseMenu.PauseMenu_C"))
  (set `self.PauseMenu` _returnvalue_2)
  (bind _returnvalue_3 (`|CreateWidget` "/Game/MyContent/HUD/GameOverMenu.GameOverMenu_C"))
  (set `self.GameOverMenu` _returnvalue_3)
  (bind _returnvalue_4 (`|CreateWidget` "/Game/MyContent/HUD/WinScreenMenu.WinScreenMenu_C"))
  (set `self.WinScreenMenu` _returnvalue_4))

(fn `UserConstructionScript`)