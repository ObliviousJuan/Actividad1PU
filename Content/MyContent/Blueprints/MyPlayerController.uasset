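; Player controller that routes Enhanced Input actions to the player's MyCharacter and handles pausing.
; It caches the character on BeginPlay, then forwards jump, look and movement along the character's right and forward vectors.
; The pause action clears all widgets, then toggles game pause, showing either the character's pause menu or its HUD.
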(event `self.ReceiveBeginPlay`
  (bind _asmy_character (cast `/Game/MyContent/Blueprints/MyCharacter` (`GameplayStatics.GetPlayerCharacter` 0)))
  (set `self.My Character` _asmy_character))

(event `EnhancedInput|/Game/MyContent/Inputs/IA_Jump`
  (params (ActionValue :type Boolean) (ElapsedSeconds :type "Float (double-precision)") (TriggeredSeconds :type "Float (double-precision)") (InputAction :type "InputAction Object Reference" :default "/Game/MyContent/Inputs/IA_Jump.IA_Jump"))
  ; Chartacter
  (:`Triggered`
    (`Character.Jump` (`self.My Character`))))

(event `EnhancedInput|/Game/MyContent/Inputs/IA_Look`
  (params (ActionValue :type "Vector2D Structure") (ElapsedSeconds :type "Float (double-precision)") (TriggeredSeconds :type "Float (double-precision)") (InputAction :type "InputAction Object Reference" :default "/Game/MyContent/Inputs/IA_Look.IA_Look"))
  (bind _my_character (`self.My Character`))
  ; Chartacter
  (:`Triggered`
    (`Pawn.AddControllerYawInput` _my_character ActionValue_X)
    (`Pawn.AddControllerPitchInput` _my_character ActionValue_Y)))

(event `EnhancedInput|/Game/MyContent/Inputs/IA_Move`
  (params (ActionValue :type "Vector2D Structure") (ElapsedSeconds :type "Float (double-precision)") (TriggeredSeconds :type "Float (double-precision)") (InputAction :type "InputAction Object Reference" :default "/Game/MyContent/Inputs/IA_Move.IA_Move"))
  (bind _my_character (`self.My Character`))
  ; Character movement
  (:`Triggered`
    (`Pawn.AddMovementInput` _my_character (`self.GetActorRightVector` _my_character) ActionValue_X false)
    (`Pawn.AddMovementInput` _my_character (`self.GetActorForwardVector` _my_character) ActionValue_Y false)))

(event `EnhancedInput|/Game/MyContent/Inputs/IA_Pause`
  (params (ActionValue :type "Vector2D Structure") (ElapsedSeconds :type "Float (double-precision)") (TriggeredSeconds :type "Float (double-precision)") (InputAction :type "InputAction Object Reference" :default "/Game/MyContent/Inputs/IA_Pause.IA_Pause"))
  (bind _my_character (`self.My Character`))
  ; Pause Game
  (:`Triggered`
    (`WidgetLayoutLibrary.RemoveAllWidgets`)
    (if (`GameplayStatics.IsGamePaused`)
      (`UserWidget.AddToViewport` (`/Game/MyContent/Blueprints/MyCharacter.MyHUD` _my_character) 0)
      (`GameplayStatics.SetGamePaused` false)
      (else
        (`UserWidget.AddToViewport` (`/Game/MyContent/Blueprints/MyCharacter.PauseMenu` _my_character) 0)
        (`GameplayStatics.SetGamePaused` true)))))

(fn `UserConstructionScript`)